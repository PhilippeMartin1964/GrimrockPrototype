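; Party pawn Blueprint for a Grimrock-style prototype that binds keyboard keys to inventory debug and test actions.
; Keys equip or unequip the selected character's main-hand item, move items between inventory slots, main hand and cursor, and toggle the inventory widget.
; Other keys log party inventory and ownership diagnostics, partly through PartyInventoryComponent.
; Two receptacle cursor-placement calls are left unwired.
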(event `Key|K`
  (params (Key :type "Key Structure"))
  (:`Pressed`
    (`self.EquipSelectedCharacterItemFromInventorySlot` 0 "MainHand")
    (`self.LogPartyInventoryDiagnostics`)))

(event `Key|L`
  (params (Key :type "Key Structure"))
  (:`Pressed`
    (`self.UnequipSelectedCharacterItemToInventory` "MainHand")
    (`self.LogPartyInventoryDiagnostics`)))

(event `Key|T`
  (params (Key :type "Key Structure"))
  (:`Pressed`
    (`self.DebugTakeInventorySlotToCursor` 0)))

(event `Key|Y`
  (params (Key :type "Key Structure"))
  (:`Pressed`
    (`self.TryEquipCursorItemToSelectedCharacterMainHand`)))

(event `Key|U`
  (params (Key :type "Key Structure"))
  (:`Pressed`
    (`self.DebugPlaceCursorItemInSelectedInventory`)))

(event `Key|O`
  (params (Key :type "Key Structure"))
  (:`Pressed`
    (`GridPartyInventoryComponent.LogInventoryOwnershipDiagnostics` (`self.PartyInventoryComponent`))))

(event `Key|P`
  (params (Key :type "Key Structure"))
  (:`Pressed`
    (`self.LogPartyInventoryDiagnostics`)))

(event `Key|I`
  (params (Key :type "Key Structure"))
  (:`Pressed`
    (`self.ToggleInventoryWidget`)))

(event `Key|M`
  (params (Key :type "Key Structure"))
  (:`Pressed`
    (`self.TryTakeSelectedCharacterMainHandToCursor`)))

(fn `UserConstructionScript`)